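; BP_Door2 is a sliding door actor that opens and closes with the E key.
; Overlapping its Box enables input for player controller 0, and ending the overlap disables it.
; The DoorMove timeline slides the Door along relative Y, playing to open and reversing to close.
; Tick derives DoorClosed by comparing the timeline value to a threshold, which decides the direction of the next press.
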(event OnComponentBeginOverlap(Box)
  (params (OverlappedComponent :type Primitive%20Component%20Object%20Reference) (OtherActor :type Actor%20Object%20Reference) (OtherComp :type Primitive%20Component%20Object%20Reference) (OtherBodyIndex :type Integer) (bFromSweep :type Boolean) (SweepResult :type Hit%20Result%20Structure%20%28by%20ref%29))
  (Input|EnableInput (Game|GetPlayerController 0)))

(event OnComponentEndOverlap(Box)
  (params (OverlappedComponent :type Primitive%20Component%20Object%20Reference) (OtherActor :type Actor%20Object%20Reference) (OtherComp :type Primitive%20Component%20Object%20Reference) (OtherBodyIndex :type Integer))
  (Input|DisableInput (Game|GetPlayerController 0)))

(event EventBeginPlay)

(event Collision|EventActorBeginOverlap
  (params (OtherActor :type Actor%20Object%20Reference)))

(event EventTick
  (params (DeltaSeconds :type Float%20%28single-precision%29))
  (Variables|Default|SetDoorClosed (< (stale Input|KeyboardEvents|E _door_2) 75.0)))

(event Input|KeyboardEvents|E
  (params (Key :type Key%20Structure :default "None"))
  (bind _door (Variables|Default|GetDoor))
  (:Pressed
    (if (Variables|Default|GetDoorClosed)
      (bind _door_2 (Timeline|DoorMove Play)
        (:Update
          (Transformation|SetRelativeLocationAndRotation _door (Math|Vector|MakeVector 0.0 _door_2 0.0) (Variables|/Script/Engine.SceneComponent|GetRelativeRotation _door) false false)))
      (else
        (Timeline|DoorMove Reverse)))))

(fn ConstructionScript)