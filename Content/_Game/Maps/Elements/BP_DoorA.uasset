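; BP_DoorA is a key-locked sliding door that the player opens and closes with F.
; Box overlap toggles the actor's input, without filtering which actor overlaps.
; F runs CheckKeys, which requires every KeyTags entry as an actor tag on the player's character and prints the first missing one.
; The DoorMove timeline slides DoorR along Y, playing or reversing by DoorClosed, which Tick derives from the timeline value.
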(event OnComponentBeginOverlap(Box)
  (params (OverlappedComponent :type Primitive%20Component%20Object%20Reference) (OtherActor :type Actor%20Object%20Reference) (OtherComp :type Primitive%20Component%20Object%20Reference) (OtherBodyIndex :type Integer) (bFromSweep :type Boolean) (SweepResult :type Hit%20Result%20Structure%20%28by%20ref%29))
  (Input|EnableInput (Game|GetPlayerController 0)))

(event OnComponentEndOverlap(Box)
  (params (OverlappedComponent :type Primitive%20Component%20Object%20Reference) (OtherActor :type Actor%20Object%20Reference) (OtherComp :type Primitive%20Component%20Object%20Reference) (OtherBodyIndex :type Integer))
  (Input|DisableInput (Game|GetPlayerController 0)))

(event EventBeginPlay)

(event Collision|EventActorBeginOverlap
  (params (OtherActor :type Actor%20Object%20Reference)))

(event EventTick
  (params (DeltaSeconds :type Float%20%28single-precision%29))
  (Variables|Default|SetDoorClosed (< (stale Input|KeyboardEvents|F _door) 75.0)))

(event Input|KeyboardEvents|F
  (params (Key :type Key%20Structure :default "None"))
  (:Pressed
    (bind _asshooter_character_bp (Utilities|Casting|CastToShooterCharacterBP (Game|GetPlayerCharacter 0)))
    (bind _haskey (CallFunction|CheckKeys _asshooter_character_bp))
    (if _haskey
      (if (Variables|Default|GetDoorClosed)
        (bind _door (Timeline|DoorMove Play)
          (:Update
            (Transformation|SetRelativeLocationAndRotation (Variables|Default|GetDoorR) (Math|Vector|MakeVector 0.0 (* _door -1.0) 0.0) "0, 0, 0" false false)))
        (else
          (Timeline|DoorMove Reverse))))))

(fn ConstructionScript)

(fn CheckKeys
  (params (Actor :type Actor%20Object%20Reference))
  (for _array_element (Variables|Key|GetKeyTags)
    (if (not (Actor|ActorHasTag Actor _array_element))
      (Development|PrintString (Utilities|String|Append "You need: " (Utilities|String|ToString(Name) _array_element)))
      (return false)))
  (return true))