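; BP_Door3 is a two-panel sliding door that the player can operate only when carrying the required key tags.
; On box overlap, CheckKeys tests the player character for every tag in Keys, printing the first missing one or enabling input if all match; end overlap disables input.
; E plays or reverses the DoorMove timeline based on DoorClosed, which Tick derives from timeline position, sliding the panels in opposite directions along X.
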(event OnComponentBeginOverlap(Box)
  (params (OverlappedComponent :type Primitive%20Component%20Object%20Reference) (OtherActor :type Actor%20Object%20Reference) (OtherComp :type Primitive%20Component%20Object%20Reference) (OtherBodyIndex :type Integer) (bFromSweep :type Boolean) (SweepResult :type Hit%20Result%20Structure%20%28by%20ref%29))
  (bind _asshooter_character_bp (Utilities|Casting|CastToShooterCharacterBP (Game|GetPlayerCharacter 0)))
  (bind _haskey (CallFunction|CheckKeys _asshooter_character_bp))
  (if _haskey
    (Input|EnableInput (Game|GetPlayerController 0))))

(event OnComponentEndOverlap(Box)
  (params (OverlappedComponent :type Primitive%20Component%20Object%20Reference) (OtherActor :type Actor%20Object%20Reference) (OtherComp :type Primitive%20Component%20Object%20Reference) (OtherBodyIndex :type Integer))
  (Input|DisableInput (Game|GetPlayerController 0)))

(event EventBeginPlay)

(event Collision|EventActorBeginOverlap
  (params (OtherActor :type Actor%20Object%20Reference)))

(event EventTick
  (params (DeltaSeconds :type Float%20%28single-precision%29))
  (Variables|Default|SetDoorClosed (< (stale Input|KeyboardEvents|E _door) 1e+02)))

(event Input|KeyboardEvents|E
  (params (Key :type Key%20Structure :default "None"))
  (:Pressed
    (if (Variables|Default|GetDoorClosed)
      (bind _door (Timeline|DoorMove Play)
        (:Update
          (Transformation|SetRelativeLocationAndRotation (Variables|Default|GetDoorL) (+ "202.491274,0.000000,-0.000002" (Math|Vector|MakeVector _door 0.0 0.0)) "0, 0, 0" false false)
          (Transformation|SetRelativeLocationAndRotation (Variables|Default|GetDoorR) (Math|Vector|MakeVector (* _door -1.0) 0.0 0.0) "0, 0, 0" false false)))
      (else
        (Timeline|DoorMove Reverse)))))

(fn ConstructionScript)

(fn CheckKeys
  (params (Actor :type Actor%20Object%20Reference))
  (for _array_element (Variables|Default|GetKeys)
    (if (not (Actor|ActorHasTag Actor _array_element))
      (Development|PrintText (Utilities|Text|ToText(Name) _array_element))
      (return false)))
  (return true))