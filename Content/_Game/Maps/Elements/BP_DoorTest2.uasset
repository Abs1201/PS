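; Test door actor that slides along its relative Y axis when E is pressed, driven by the DoorMove timeline.
; E plays or reverses the timeline based on IsDoorClosed, which Tick recomputes from the track value against a threshold.
; Leaving the Box trigger disables player input, but entering does nothing because the EnableInput node is unconnected.
; A debug "Hello" prints when opening.
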(event OnComponentBeginOverlap(Box)
  (params (OverlappedComponent :type Primitive%20Component%20Object%20Reference) (OtherActor :type Actor%20Object%20Reference) (OtherComp :type Primitive%20Component%20Object%20Reference) (OtherBodyIndex :type Integer) (bFromSweep :type Boolean) (SweepResult :type Hit%20Result%20Structure%20%28by%20ref%29)))

(event OnComponentEndOverlap(Box)
  (params (OverlappedComponent :type Primitive%20Component%20Object%20Reference) (OtherActor :type Actor%20Object%20Reference) (OtherComp :type Primitive%20Component%20Object%20Reference) (OtherBodyIndex :type Integer))
  (Input|DisableInput (Game|GetPlayerController 0)))

(event EventBeginPlay)

(event Collision|EventActorBeginOverlap
  (params (OtherActor :type Actor%20Object%20Reference)))

(event EventTick
  (params (DeltaSeconds :type Float%20%28single-precision%29))
  (Variables|Default|SetbIsDoorClosed (< (stale Input|KeyboardEvents|E _newtrack_0) 1e+02)))

(event Input|KeyboardEvents|E
  (params (Key :type Key%20Structure :default "None"))
  (:Pressed
    (if (Variables|Default|GetbIsDoorClosed)
      (Development|PrintString "Hello")
      (bind _newtrack_0 (Timeline|DoorMove Play)
        (:Update
          (Transformation|SetRelativeLocation (Variables|Default|GetDoor) (Math|Vector|MakeVector 0.0 (* _newtrack_0 -1.0) 0.0) false false)))
      (else
        (Timeline|DoorMove Reverse)))))

(fn ConstructionScript)