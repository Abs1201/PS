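; BP_EnemyShooterBoss is a shooter boss enemy that adds health bar handling and a proximity wake-up on top of its parent class.
; On BeginPlay it links its health bar widget to itself and hides it.
; Show and hide events toggle that widget's visibility, with only the show event also calling the parent.
; A ShooterCharacterBP entering WakeUpBox sets the IsWakeUp flag.
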(event OnComponentBeginOverlap(WakeUpBox)
  (params (OverlappedComponent :type Primitive%20Component%20Object%20Reference) (OtherActor :type Actor%20Object%20Reference) (OtherComp :type Primitive%20Component%20Object%20Reference) (OtherBodyIndex :type Integer) (bFromSweep :type Boolean) (SweepResult :type Hit%20Result%20Structure%20%28by%20ref%29))
  (Utilities|Casting|CastToShooterCharacterBP OtherActor)
  (Variables|Default|SetbIsWakeUp self true))

(event EventBeginPlay
  (bind _asenemy_health_bar_bp (Utilities|Casting|CastToEnemyHealthBarBP (UserInterface|GetUserWidgetObject (Variables|Default|GetHealthBar))))
  (Variables|/Game/_Game/HUD/EnemyHealthBarBP.EnemyHealthBarBP_C|SetEnemy _asenemy_health_bar_bp self)
  (Widget|SetVisibility (UserInterface|GetUserWidgetObject (Variables|Default|GetHealthBar)) "Hidden"))

(event Collision|EventActorBeginOverlap
  (params (OtherActor :type Actor%20Object%20Reference)))

(event EventTick
  (params (DeltaSeconds :type Float%20%28single-precision%29)))

(event EventShowHealthBar
  (Widget|SetVisibility (UserInterface|GetUserWidgetObject (Variables|Default|GetHealthBar)) "Visible")
  (|CallParentFunction))

(event EventHideHealthBar
  (Widget|SetVisibility (UserInterface|GetUserWidgetObject (Variables|Default|GetHealthBar)) "Hidden"))

(fn ConstructionScript)