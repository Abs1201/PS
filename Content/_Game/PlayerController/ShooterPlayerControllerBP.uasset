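; Player controller for the shooter that handles the menu and inventory hotkeys.
; On BeginPlay it fetches and caches the shooter HUD through a setup helper with a delay or timeout value.
; Escape spawns a new settings widget on screen, while I and O ask the cached HUD to toggle the inventory and weapon inventory.
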(event EventBeginPlay
  (bind _asshooter_hudbp (Utilities|GetShooterHUDBPSetup 4.0)
    (:Success
      (Variables|Default|SetAs%20Shooter%20HUDBP _asshooter_hudbp))))

(event EventTick
  (params (DeltaSeconds :type Float%20%28single-precision%29)))

(event Input|KeyboardEvents|Escape
  (params (Key :type Key%20Structure :default "None"))
  (:Pressed
    (bind _returnvalue (UserInterface|CreateWidget "/Game/_Game/HUD/WBP_Setting.WBP_Setting_C"))
    (UserInterface|Viewport|AddtoViewport _returnvalue 0)))

(event Input|KeyboardEvents|I
  (params (Key :type Key%20Structure :default "None"))
  (:Pressed
    (Default|ToggleInventory (Variables|Default|GetAs%20Shooter%20HUDBP))))

(event Input|KeyboardEvents|O
  (params (Key :type Key%20Structure :default "None"))
  (:Pressed
    (Default|ToggleWeaponInventory (Variables|Default|GetAs%20Shooter%20HUDBP))))

(fn ConstructionScript)